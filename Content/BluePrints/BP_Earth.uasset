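; BP_Earth is the Earth actor that enemy ships damage on contact, with game over when its health runs out.
; On BeginPlay it adds the game screen widget to the viewport.
; Overlaps with BP_EnemyShip or Enemy_F, matched by exact class, subtract a fixed amount of health and destroy the enemy.
; At zero health or below, it pauses the game after a short delay and shows the game over widget.
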(event EventBeginPlay
  (bind _returnvalue (UserInterface|CreateWidget "/Game/BluePrints/HUD/WBP_GameScreen.WBP_GameScreen_C"))
  (UserInterface|Viewport|AddtoViewport _returnvalue 0))

(event Collision|EventActorBeginOverlap
  (params (OtherActor :type Actor%20Object%20Reference))
  (if (or (== (Utilities|GetClass OtherActor) "/Game/BluePrints/Ships/BP_EnemyShip.BP_EnemyShip_C") (== (Utilities|GetClass OtherActor) "/Game/BluePrints/Ships/Enemy_F.Enemy_F_C"))
    (bind _output_get (Variables|Default|Sethealth (- (Variables|Default|Gethealth) 45.0)))
    (Actor|DestroyActor OtherActor)
    (if (<= _output_get 0.0)
      (Utilities|FlowControl|Delay 0.5)
      (Game|SetGamePaused true)
      (bind _returnvalue (UserInterface|CreateWidget "/Game/BluePrints/HUD/WBP_GameOver.WBP_GameOver_C"))
      (UserInterface|Viewport|AddtoViewport _returnvalue 0))))

(fn ConstructionScript)