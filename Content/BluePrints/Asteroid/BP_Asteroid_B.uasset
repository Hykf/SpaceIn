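; Large asteroid actor that ends the game on overlapping BP_Earth by pausing and showing the game-over widget.
; Any other overlap plays audio and reduces Health; at zero it plays audio, spawns two randomly rotated BP_Asteroid_M fragments at its location and destroys itself.
; The construction script randomizes mesh rotation, and BeginPlay starts a timed self-destruct after a fixed delay.
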(event EventBeginPlay
  (Utilities|FlowControl|Delay 45.0)
  (Actor|DestroyActor))

(event Collision|EventActorBeginOverlap
  (params (OtherActor :type Actor%20Object%20Reference))
  (bind _returnvalue (Math|Random|RandomFloatinRange 0.0 1.8e+02))
  (bind _returnvalue_2 (Math|Random|RandomFloatinRange 0.0 1.8e+02))
  (if (== (Utilities|GetClass OtherActor) "/Game/BluePrints/BP_Earth.BP_Earth_C")
    (Game|SetGamePaused true)
    (bind _returnvalue_3 (UserInterface|CreateWidget "/Game/BluePrints/HUD/WBP_GameOver.WBP_GameOver_C"))
    (UserInterface|Viewport|AddtoViewport _returnvalue_3 0)
    (else
      (AddComponent|AddAudioComponent false)
      (bind _output_get (Variables|Default|Sethealth (- (Variables|Default|Gethealth) 1e+01)))
      (if (<= _output_get 0.0)
        (AddComponent|AddAudioComponent false)
        (Game|SpawnActorfromClass "/Game/BluePrints/Asteroid/BP_Asteroid_M.BP_Asteroid_M_C" (Math|Transform|MakeTransform (.location (Transformation|GetActorTransform)) (Math|Rotator|MakeRotator _returnvalue_2 0.0 _returnvalue_2) "1.000000,1.000000,1.000000") "AdjustIfPossibleButAlwaysSpawn" 0 0)
        (Game|SpawnActorfromClass "/Game/BluePrints/Asteroid/BP_Asteroid_M.BP_Asteroid_M_C" (Math|Transform|MakeTransform (.location (Transformation|GetActorTransform)) (Math|Rotator|MakeRotator _returnvalue 0.0 _returnvalue) "1.000000,1.000000,1.000000") "AdjustIfPossibleButAlwaysSpawn" 0 0)
        (Actor|DestroyActor)))))

(fn ConstructionScript
  (Transformation|SetWorldRotation (Variables|Default|GetStaticMeshComponent) (Math|Random|RandomRotator false) false false))

(fn AsteroidSettings
  (return "0, 0, 0" 0.0 0.0))