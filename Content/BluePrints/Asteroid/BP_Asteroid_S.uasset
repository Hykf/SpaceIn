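; BP_Asteroid_S is an asteroid actor, likely the small variant, that ends the game if it reaches Earth.
; Overlapping BP_Earth pauses the game and shows the WBP_GameOver widget.
; Any other overlap subtracts health and destroys the asteroid once health runs out.
; The construction script gives its mesh a random rotation, and a delay from BeginPlay destroys it after a fixed lifetime.
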(event EventBeginPlay
  (Utilities|FlowControl|Delay 55.0)
  (Actor|DestroyActor))

(event Collision|EventActorBeginOverlap
  (params (OtherActor :type Actor%20Object%20Reference))
  (if (== (Utilities|GetClass OtherActor) "/Game/BluePrints/BP_Earth.BP_Earth_C")
    (Game|SetGamePaused true)
    (bind _returnvalue (UserInterface|CreateWidget "/Game/BluePrints/HUD/WBP_GameOver.WBP_GameOver_C"))
    (UserInterface|Viewport|AddtoViewport _returnvalue 0)
    (else
      (bind _output_get (Variables|Default|Sethealth (- (Variables|Default|Gethealth) 1e+01)))
      (if (<= _output_get 0.0)
        (Actor|DestroyActor)))))

(fn ConstructionScript
  (Transformation|SetWorldRotation (Variables|Default|GetStaticMeshComponent) (Math|Random|RandomRotator false) false false))