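; Asteroid spawner actor that continually creates small, medium or big asteroids at random points inside its Box volume.
; Tick runs a randomized Delay scaled by frame time, then picks one of the three asteroid classes with equal odds.
; AsteroidSettings supplies the spawn location and derives roll and yaw from the player pawn's world position vector, adding a large random offset to yaw.
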(event EventTick
  (params (DeltaSeconds :type Float%20%28single-precision%29))
  (Utilities|FlowControl|Delay (* DeltaSeconds (Math|Random|RandomFloatinRange 1.0 1e+02)))
  (switch int (Math|Random|RandomIntegerinRange 0 2)
    (:0
      (bind (_returnvalue _returnvalue_roll _returnvalue2) (CallFunction|AsteroidSettings))
      (Game|SpawnActorfromClass "/Game/BluePrints/Asteroid/BP_Asteroid_S.BP_Asteroid_S_C" (Math|Transform|MakeTransform _returnvalue (Math|Rotator|MakeRotator _returnvalue_roll 0.0 _returnvalue2) "1.000000,1.000000,1.000000") "Undefined" 0 0))
    (:1
      (bind (_returnvalue_2 _returnvalue_roll_2 _returnvalue2_2) (CallFunction|AsteroidSettings))
      (Game|SpawnActorfromClass "/Game/BluePrints/Asteroid/BP_Asteroid_M.BP_Asteroid_M_C" (Math|Transform|MakeTransform _returnvalue_2 (Math|Rotator|MakeRotator _returnvalue_roll_2 0.0 _returnvalue2_2) "1.000000,1.000000,1.000000") "Undefined" 0 0))
    (:2
      (bind (_returnvalue_3 _returnvalue_roll_3 _returnvalue2_3) (CallFunction|AsteroidSettings))
      (Game|SpawnActorfromClass "/Game/BluePrints/Asteroid/BP_Asteroid_B.BP_Asteroid_B_C" (Math|Transform|MakeTransform _returnvalue_3 (Math|Rotator|MakeRotator _returnvalue_roll_3 0.0 _returnvalue2_3) "1.000000,1.000000,1.000000") "Undefined" 0 0))))

(fn ConstructionScript)

(fn AsteroidSettings
  (bind _returnvalue (Game|Player|GetPlayerPawn 0))
  (bind _returnvalue_2 (Transformation|GetActorLocation _returnvalue))
  (bind _returnvalue_3 (Math|Conversions|RotationFromXVector _returnvalue_2))
  (return (Math|Random|RandomPointinBoundingBox (Transformation|GetWorldLocation (Variables|Default|GetDefaultSceneRoot)) (Variables|/Script/Engine.BoxComponent|GetBoxExtent (Variables|Default|GetBox))) (.roll _returnvalue_3) (+ (.yaw _returnvalue_3) (Math|Random|RandomFloatinRange 4.0 4e+03))))