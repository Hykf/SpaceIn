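; Enemy_F is an enemy ship that fires projectiles at random intervals and dies when hit by a player projectile.
; Tick runs into a random Delay of up to 20 seconds, which acts as the fire timer before spawning BP_Projectile_Enemy at the Arrow component's location and rotation.
; On overlap with an actor whose class is exactly BP_Projectile_Player, the ship destroys itself.
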(event Collision|EventActorBeginOverlap
  (params (OtherActor :type Actor%20Object%20Reference))
  (if (== (Utilities|GetClass OtherActor) "/Game/BluePrints/Projectile/BP_Projectile_Player.BP_Projectile_Player_C")
    (Actor|DestroyActor)))

(event EventTick
  (params (DeltaSeconds :type Float%20%28single-precision%29))
  (bind _arrow (Variables|Default|GetArrow))
  (Utilities|FlowControl|Delay (* (Math|Random|RandomFloat) 2e+01))
  (Game|SpawnActorfromClass "/Game/BluePrints/Projectile/BP_Projectile_Enemy.BP_Projectile_Enemy_C" (Math|Transform|MakeTransform (Transformation|GetSocketLocation _arrow "None") (Transformation|GetSocketRotation _arrow "None")) "Undefined" self 0))

(fn ConstructionScript)