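; Enemy formation "orbit" actor that slides a row of enemy ship components back and forth along a spline.
; Tick advances the lead distance by Speed, spaces followers by a fixed offset, and reverses when either end passes the spline's limits.
; Delayed branches periodically flip Speed, boosting it by Orbita_Wrogowie actor count, and step the actor's scale down and position along -Y as an approach.
; The shrink-then-destroy logic is unconnected.
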(event EventTick
  (params (DeltaSeconds :type Float%20%28single-precision%29))
  (bind _self self)
  (bind _ostatni (Variables|Default|GetOstatni))
  (bind _dist_pierwszy (Variables|Default|GetDist_Pierwszy))
  (bind _spline (Variables|Default|GetSpline))
  (bind _pierwszy_ (Variables|Default|GetPierwszy%20))
  (bind _returnvalue (Transformation|GetActorScale3D _self))
  (bind _returnvalue_2 (Spline|GetTransformatDistanceAlongSpline _spline _dist_pierwszy "Local" true))
  (Utilities|FlowControl|Sequence
    (:then_0
      ;[1 1 1] Zmiana kierunku i predkosci
      (Utilities|FlowControl|Delay (Math|Random|RandomFloatinRange 1e+01 3e+01))
      (Variables|Default|SetSpeed (* (Variables|Default|GetSpeed) -1.0))
      (bind _outactors (Actor|GetAllActorsOfClass "/Game/BluePrints/Ships/Orbita_Wrogowie.Orbita_Wrogowie_C"))
      (Variables|Default|SetSpeed (- (Variables|Default|GetSpeed) (* (Utilities|Array|Length _outactors) -25))))
    (:then_1
      (bind _do_dist_ostatni (CallFunction|SETDist DeltaSeconds))
      (Variables|Default|SetDist_Ostatni _do_dist_ostatni)
      (Utilities|FlowControl|Sequence
        (:then_0
          ;[1 1 1] BACK
          (Transformation|SetRelativeTransform _pierwszy_ (Math|Transform|MakeTransform (.location _returnvalue_2) (.rotation _returnvalue_2) (Variables|/Script/Engine.SceneComponent|GetRelativeScale3D _pierwszy_)) false false)
          (if (not (> (Variables|Default|GetDist_Pierwszy) (Spline|GetSplineLength (Variables|Default|GetSpline))))
            (if (< (Variables|Default|GetDist_Pierwszy) 0.0)
              (Variables|Default|SetSpeed (* (Variables|Default|GetSpeed) -1.0)))))
        (:then_1
          (CallFunction|SETUPBETWEEN))
        (:then_2
          ;[1 1 1] FRONT
          (Transformation|SetRelativeTransform _ostatni (Math|Transform|MakeTransform (.location (Spline|GetTransformatDistanceAlongSpline (Variables|Default|GetSpline) (Variables|Default|GetDist_Ostatni) "Local" true)) (.rotation (Spline|GetTransformatDistanceAlongSpline (Variables|Default|GetSpline) (Variables|Default|GetDist_Ostatni) "Local" true)) (Variables|/Script/Engine.SceneComponent|GetRelativeScale3D _ostatni)) false false)
          (if (> (Variables|Default|GetDist_Ostatni) (Spline|GetSplineLength (Variables|Default|GetSpline)))
            (Variables|Default|SetSpeed (* (Variables|Default|GetSpeed) -1.0))))))
    (:then_2
      ;[1 1 1] Przyblizanie SIe
      (if (Utilities|Operators|EqualEqual _returnvalue "2.000000,2.000000,2.000000" 0.5)
        (Transformation|SetActorScale3D (- _returnvalue "2.000000,2.000000,2.000000"))
        (else
          (Utilities|FlowControl|Delay 2e+01)
          (Transformation|SetActorScale3D (- _returnvalue "1.000000,1.000000,1.000000"))))
      (Transformation|SetActorLocation (- (Transformation|GetActorLocation _self) "0,500.000000,0") false false))))

(fn ConstructionScript)

(fn SETDist
  (params (Dist :type Float%20%28double-precision%29))
  (bind _output_get (Variables|Default|SetDist_Pierwszy (+ (* Dist (Variables|Default|GetSpeed)) (Variables|Default|GetDist_Pierwszy))))
  (bind _output_get_2 (Variables|Default|SetDist2 (+ _output_get (Variables|Default|GetDODANA))))
  (bind _output_get_3 (Variables|Default|SetDist3 (+ _output_get_2 (Variables|Default|GetDODANA))))
  (bind _output_get_4 (Variables|Default|SetDist4 (+ _output_get_3 (Variables|Default|GetDODANA))))
  (bind _output_get_5 (Variables|Default|SetDist5 (+ _output_get_4 (Variables|Default|GetDODANA))))
  (bind _output_get_6 (Variables|Default|SetDist%206 (+ _output_get_5 (Variables|Default|GetDODANA))))
  (bind _output_get_7 (Variables|Default|SetDist%207 (+ _output_get_6 (Variables|Default|GetDODANA))))
  (bind _output_get_8 (Variables|Default|SetDist%208 (+ _output_get_7 (Variables|Default|GetDODANA))))
  (bind _output_get_9 (Variables|Default|SetDist%209 (+ _output_get_8 (Variables|Default|GetDODANA))))
  (bind _output_get_10 (Variables|Default|SetDist%2010 (+ _output_get_9 (Variables|Default|GetDODANA))))
  (return _output_get_10))

(fn ADDtoSpline
  (params (Target :type Scene%20Component%20Object%20Reference) (Distance :type Float%20%28single-precision%29))
  (bind _spline (Variables|Default|GetSpline))
  (bind _returnvalue (Spline|GetTransformatDistanceAlongSpline _spline Distance "Local" true))
  (Transformation|SetRelativeTransform Target (Math|Transform|MakeTransform (.location _returnvalue) (.rotation _returnvalue) (Variables|/Script/Engine.SceneComponent|GetRelativeScale3D Target)) false false))

(fn SETUPBETWEEN
  (CallFunction|ADDtoSpline (Variables|Default|GetE1_Same_Testy) (Variables|Default|GetDist2))
  (CallFunction|ADDtoSpline (Variables|Default|GetE1_Same_Testy1) (Variables|Default|GetDist3))
  (CallFunction|ADDtoSpline (Variables|Default|GetE1_Same_Testy2) (Variables|Default|GetDist4))
  (CallFunction|ADDtoSpline (Variables|Default|GetE1_Same_Testy3) (Variables|Default|GetDist5))
  (CallFunction|ADDtoSpline (Variables|Default|GetE1_Same_Testy4) (Variables|Default|GetDist%206))
  (CallFunction|ADDtoSpline (Variables|Default|GetE1_Same_Testy5) (Variables|Default|GetDist%207))
  (CallFunction|ADDtoSpline (Variables|Default|GetE1_Same_Testy6) (Variables|Default|GetDist%208))
  (CallFunction|ADDtoSpline (Variables|Default|GetE1_Same_Testy7) (Variables|Default|GetDist%209))
  (CallFunction|ADDtoSpline (Variables|Default|GetE1_Same_Testy8) (Variables|Default|GetDist%2010)))