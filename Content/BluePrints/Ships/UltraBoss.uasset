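; UltraBoss is a boss ship Blueprint that travels along a spline and can be destroyed through overlap hits.
; Each Tick adds speed times delta time to a distance, then sets Sphere1's relative location and rotation from that spline point.
; Passing the spline's end pauses the game.
; Any actor overlap subtracts a fixed amount of health, destroying the boss once health runs out.
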(event EventBeginPlay)

(event Collision|EventActorBeginOverlap
  (params (OtherActor :type Actor%20Object%20Reference))
  ;[1 1 1] Dostawanie obrazen
  (bind _output_get (Variables|Default|SetHealth (- (Variables|Default|GetHealth) 1e+01)))
  (if (<= _output_get 0.0)
    (Actor|DestroyActor)))

(event EventTick
  (params (DeltaSeconds :type Float%20%28single-precision%29))
  (bind _sphere1 (Variables|Default|GetSphere1))
  ;[1 0 0.08657] RUCH
  (Variables|Default|SetDist (+ (* DeltaSeconds (Variables|Default|GetSpeed)) (Variables|Default|GetDist)))
  (Transformation|SetRelativeTransform _sphere1 (Math|Transform|MakeTransform (.location (Spline|GetTransformatDistanceAlongSpline (Variables|Default|GetSpline) (Variables|Default|GetDist) "Local" false)) (.rotation (Spline|GetTransformatDistanceAlongSpline (Variables|Default|GetSpline) (Variables|Default|GetDist) "Local" false)) (Variables|/Script/Engine.SceneComponent|GetRelativeScale3D _sphere1)) false false)
  (if true
    (if (> (Variables|Default|GetDist) (Spline|GetSplineLength (Variables|Default|GetSpline)))
      (Game|SetGamePaused true))))

(fn ConstructionScript)