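; BP_PlayerShip is the player's ship, which circles an orbit path and ends the game when it overlaps another actor.
; Each tick advances a distance by Speed and moves the sphere component to the matching spline location and rotation, keeping its scale.
; The distance wraps at both ends of the spline, so travel loops in either direction.
; Any overlap pauses the game and shows the WBP_GameOver widget.
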(event Collision|EventActorBeginOverlap
  (params (OtherActor :type Actor%20Object%20Reference))
  ;[0 0 0] Smierc
  (Game|SetGamePaused true)
  (bind _returnvalue (UserInterface|CreateWidget "/Game/BluePrints/HUD/WBP_GameOver.WBP_GameOver_C"))
  (UserInterface|Viewport|AddtoViewport _returnvalue 0))

(event EventTick
  (params (DeltaSeconds :type Float%20%28single-precision%29))
  (bind _spherecomponent (Variables|Default|GetSphereComponent))
  ;[0.1693 1 0] Poruszanie sie po orbicie
  (Variables|Default|SetDist (+ (* DeltaSeconds (Variables|Default|GetSpeed)) (Variables|Default|GetDist)))
  (Transformation|SetRelativeTransform _spherecomponent (Math|Transform|MakeTransform (.location (Spline|GetTransformatDistanceAlongSpline (Variables|Default|GetSplineComponent) (Variables|Default|GetDist) "Local" false)) (.rotation (Spline|GetTransformatDistanceAlongSpline (Variables|Default|GetSplineComponent) (Variables|Default|GetDist) "Local" false)) (Variables|/Script/Engine.SceneComponent|GetRelativeScale3D _spherecomponent)) false false)
  (if true
    (if (> (Variables|Default|GetDist) (Spline|GetSplineLength (Variables|Default|GetSplineComponent)))
      (Variables|Default|SetDist 0.0)
      (elif (< (Variables|Default|GetDist) 0.0)
        (Variables|Default|SetDist (Spline|GetSplineLength (Variables|Default|GetSplineComponent)))))))

(fn ConstructionScript)