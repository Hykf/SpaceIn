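; SetE is a test actor that moves a formation of five components (E1Pierwszy through E1Ostatni) along its spline.
; Tick advances a distance by Speed and places each component at evenly offset spline distances.
; When the first passes the end, the actor reverses Speed, shrinks, then destroys itself near unit scale or shifts along Y.
; The last also reverses Speed past the end, through an immediately reset DoOnce; low distances wrap to the end.
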(event EventTick
  (params (DeltaSeconds :type Float%20%28single-precision%29))
  (bind _self self)
  (bind _e1_same3 (Variables|Default|GetE1_Same3))
  (bind _e1_pierwszy (Variables|Default|GetE1_Pierwszy))
  (bind _spline (Variables|Default|GetSpline))
  (bind _e1_same1 (Variables|Default|GetE1_Same1))
  (bind _e1_same2 (Variables|Default|GetE1_Same2))
  (bind _e1_ostatni (Variables|Default|GetE1_Ostatni))
  (bind _output_get (Variables|Default|SetDist (+ (* DeltaSeconds (Variables|Default|GetSpeed)) (Variables|Default|GetDist))))
  (bind _output_get_2 (Variables|Default|SetDist1 (+ _output_get 3.5e+02)))
  (bind _output_get_3 (Variables|Default|SetDist2 (+ _output_get_2 3.5e+02)))
  (bind _output_get_4 (Variables|Default|SetDist3 (+ _output_get_3 3.5e+02)))
  (Variables|Default|SetDist4 (+ _output_get_4 3.5e+02))
  (Utilities|FlowControl|Sequence
    (:then_0
      ;[1 1 1] Comment
      (Transformation|SetRelativeTransform _e1_pierwszy (Math|Transform|MakeTransform (.location (Spline|GetTransformatDistanceAlongSpline (Variables|Default|GetSpline) (Variables|Default|GetDist) "Local" true)) (.rotation (Spline|GetTransformatDistanceAlongSpline (Variables|Default|GetSpline) (Variables|Default|GetDist) "Local" true)) (Variables|/Script/Engine.SceneComponent|GetRelativeScale3D _e1_pierwszy)) false false)
      (if true
        (if (> (Variables|Default|GetDist) (Spline|GetSplineLength _spline))
          (Variables|Default|SetDist 1.0)
          (Variables|Default|SetSpeed (* (Variables|Default|GetSpeed) -1.0))
          ;[1 0 0] Jeszcze trzeba dodac znikanie BO to dziala
          (Transformation|SetActorScale3D (- (Transformation|GetActorScale3D _self) "1.000000,1.000000,1.000000"))
          (if (Utilities|Operators|EqualEqual (Transformation|GetActorScale3D) "1.000000,1.000000,1.000000" 0.5)
            (Actor|DestroyActor)
            (else
              (Transformation|SetActorLocation (- (Transformation|GetActorLocation _self) "0,500.000000,0") false false)))
          (elif (< (Variables|Default|GetDist) 1e+01)
            (Variables|Default|SetDist (Spline|GetSplineLength _spline))))))
    (:then_1
      ;[1 1 1] Comment
      (Transformation|SetRelativeTransform _e1_same1 (Math|Transform|MakeTransform (.location (Spline|GetTransformatDistanceAlongSpline (Variables|Default|GetSpline) (Variables|Default|GetDist1) "Local" true)) (.rotation (Spline|GetTransformatDistanceAlongSpline (Variables|Default|GetSpline) (Variables|Default|GetDist1) "Local" true)) (Variables|/Script/Engine.SceneComponent|GetRelativeScale3D _e1_same1)) false false))
    (:then_2
      ;[1 1 1] Comment
      (Transformation|SetRelativeTransform _e1_same2 (Math|Transform|MakeTransform (.location (Spline|GetTransformatDistanceAlongSpline (Variables|Default|GetSpline) (Variables|Default|GetDist2) "Local" true)) (.rotation (Spline|GetTransformatDistanceAlongSpline (Variables|Default|GetSpline) (Variables|Default|GetDist2) "Local" true)) (Variables|/Script/Engine.SceneComponent|GetRelativeScale3D _e1_same2)) false false))
    (:then_3
      ;[1 1 1] Comment
      (Transformation|SetRelativeTransform _e1_same3 (Math|Transform|MakeTransform (.location (Spline|GetTransformatDistanceAlongSpline (Variables|Default|GetSpline) (Variables|Default|GetDist3) "Local" true)) (.rotation (Spline|GetTransformatDistanceAlongSpline (Variables|Default|GetSpline) (Variables|Default|GetDist3) "Local" true)) (Variables|/Script/Engine.SceneComponent|GetRelativeScale3D _e1_same3)) false false))
    (:then_5
      ;[1 1 1] Comment
      (Transformation|SetRelativeTransform _e1_ostatni (Math|Transform|MakeTransform (.location (Spline|GetTransformatDistanceAlongSpline (Variables|Default|GetSpline) (Variables|Default|GetDist4) "Local" true)) (.rotation (Spline|GetTransformatDistanceAlongSpline (Variables|Default|GetSpline) (Variables|Default|GetDist4) "Local" true)) (Variables|/Script/Engine.SceneComponent|GetRelativeScale3D _e1_ostatni)) false false)
      (if true
        (if (> (Variables|Default|GetDist4) (Spline|GetSplineLength (Variables|Default|GetSpline)))
          (Utilities|FlowControl|DoOnce false :!label _label
            (:Completed
              (Variables|Default|SetSpeed (* (Variables|Default|GetSpeed) -1.0))
              (goto _label Reset))))))))

(fn ConstructionScript)