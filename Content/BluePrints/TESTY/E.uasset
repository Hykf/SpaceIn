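; Test actor that moves a Sphere along a Spline while spawning Projectiles from an Arrow.
; Tick advances distance by Speed and places the Sphere at that spline point.
; Delays in Tick act as repeating timers, firing at random intervals up to five seconds and periodically reversing Speed.
; When NewVar0 is set, passing the end reverses Speed, while passing the start wraps to the end, both printing debug text.
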(event EventTick
  (params (DeltaSeconds :type Float%20%28single-precision%29))
  (bind _arrow (Variables|Default|GetArrow))
  (bind _spline (Variables|Default|GetSpline))
  (bind _sphere (Variables|Default|GetSphere))
  (Utilities|FlowControl|Sequence
    (:then_0
      (Utilities|FlowControl|Delay (* (Math|Random|RandomFloat) 5.0))
      (Game|SpawnActorfromClass "/Game/BluePrints/TESTY/projectile.projectile_C" (Math|Transform|MakeTransform (Transformation|GetSocketLocation _arrow "None") (Transformation|GetSocketRotation _arrow "None")) "Undefined" self 0))
    (:then_1
      (Variables|Default|SetDist (+ (* DeltaSeconds (Variables|Default|GetSpeed)) (Variables|Default|GetDist)))
      (Transformation|SetRelativeTransform _sphere (Math|Transform|MakeTransform (.location (Spline|GetTransformatDistanceAlongSpline (Variables|Default|GetSpline) (Variables|Default|GetDist) "Local" true)) (.rotation (Spline|GetTransformatDistanceAlongSpline (Variables|Default|GetSpline) (Variables|Default|GetDist) "Local" true)) (Variables|/Script/Engine.SceneComponent|GetRelativeScale3D _sphere)) false false)
      (if (Variables|Default|GetNewVar_0)
        (if (> (Variables|Default|GetDist) (Spline|GetSplineLength _spline))
          (Variables|Default|SetSpeed (* (Variables|Default|GetSpeed) -1.0))
          (Development|PrintString "DOJECHALEM DO KONCA 
")
          (elif (< (Variables|Default|GetDist) 0.0)
            (Variables|Default|SetDist (Spline|GetSplineLength _spline))
            (Development|PrintString "DOJECHALEM DO POCZATKU")))))
    (:then_2
      (Utilities|FlowControl|Delay 5.0)
      (Variables|Default|SetSpeed (* (Variables|Default|GetSpeed) -1.0)))))

(fn ConstructionScript)