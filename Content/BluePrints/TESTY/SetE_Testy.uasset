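; Test actor (SetE_Testy) that moves its E1SameTesty1 component along a spline every Tick, keeping the component's scale.
; Distance advances by Speed, which reverses past the spline's end, while a distance below zero wraps to the end.
; A Tick-driven FlipFlop feeds 5- and 7-second Delays that also reverse Speed.
; Unconnected leftovers hold earlier single-sphere and spaced five-piece followers, plus a shrink-and-destroy experiment.
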(event EventTick
  (params (DeltaSeconds :type Float%20%28single-precision%29))
  (bind _spline (Variables|Default|GetSpline))
  (bind _e1_same_testy1 (Variables|Default|GetE1_Same_Testy1))
  (Utilities|FlowControl|Sequence
    (:then_0
      (Utilities|FlowControl|FlipFlop
        (:A
          (Utilities|FlowControl|Delay 5.0))
        (:B
          (Utilities|FlowControl|Delay 7.0)))
      (Variables|Default|SetSpeed (* (Variables|Default|GetSpeed) -1.0)))
    (:then_1
      (Variables|Default|SetDist (+ (* DeltaSeconds (Variables|Default|GetSpeed)) (Variables|Default|GetDist)))
      (Transformation|SetRelativeTransform _e1_same_testy1 (Math|Transform|MakeTransform (.location (Spline|GetTransformatDistanceAlongSpline (Variables|Default|GetSpline) (Variables|Default|GetDist) "Local" true)) (.rotation (Spline|GetTransformatDistanceAlongSpline (Variables|Default|GetSpline) (Variables|Default|GetDist) "Local" true)) (Variables|/Script/Engine.SceneComponent|GetRelativeScale3D _e1_same_testy1)) false false)
      (if true
        (if (> (Variables|Default|GetDist) (Spline|GetSplineLength _spline))
          (Variables|Default|SetSpeed (* (Variables|Default|GetSpeed) -1.0))
          (elif (< (Variables|Default|GetDist) 0.0)
            (Variables|Default|SetDist (Spline|GetSplineLength _spline))))))))

(fn ConstructionScript)